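; Boomerang projectile actor that homes toward a target component and can be caught by the player.
; SetHomingTarget points its ProjectileMovement at the target, and Tick spins the actor while it is in the air.
; Any hit stops the spin, and hitting something other than the target flags HitObject.
; Reaching the target destroys the boomerang, calling CaughtBoomerang on the BoomerangNew player object only if nothing else was hit first.
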(event `self.ReceiveTick`
  (params (DeltaSeconds :type "Float (single-precision)"))
  (if (`self.inAir`)
    (`self.K2_AddActorLocalRotation` (struct :`Yaw` 5.0))))

(event `self.ReceiveBeginPlay`)

(event `self.ReceiveHit`
  (params (MyComp :type "PrimitiveComponent Object Reference") (Other :type "Actor Object Reference") (OtherComp :type "PrimitiveComponent Object Reference") (bSelfMoved :type Boolean) (HitLocation :type "Vector Structure") (HitNormal :type "Vector Structure") (NormalImpulse :type "Vector Structure") (Hit :type "HitResult Structure (by ref)"))
  (set `self.inAir` false)
  (if (== OtherComp (`self.homingTarget`))
    (if (`self.hitObject`)
      (`self.K2_DestroyActor`)
      (else
        (bind _asboomerang_new (cast `/Game/Blueprints/Boomerang/BoomerangNew` (`self.PlayerObject`)))
        (`/Game/Blueprints/Boomerang/BoomerangNew.CaughtBoomerang` _asboomerang_new)
        (`self.K2_DestroyActor`)))
    (else
      (set `self.hitObject` true))))

(fn `SetHomingTarget`
  (params (homingTarget :type "SceneComponent Object Reference"))
  (bind _output_get (set `ProjectileMovementComponent.HomingTargetComponent` homingTarget (`self.ProjectileMovement`)))
  (set `self.homingTarget` _output_get))

(fn `UserConstructionScript`)