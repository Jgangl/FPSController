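; AsheBomb is an unfinished bomb actor whose active logic only prints debug output.
; Overlap begin and end events print the other actor's name, and Explode prints the count of overlapping components.
; Disconnected nodes hold the intended behavior: tracking physics-simulating objects in ObjectsInRange and applying a linear-falloff radial impulse to overlapping components from the bomb's location.
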(event `self.ReceiveActorBeginOverlap`
  (params (OtherActor :type "Actor Object Reference"))
  ;[1 1 1] Comment
  (`KismetSystemLibrary.PrintString` (`KismetSystemLibrary.GetDisplayName` OtherActor)))

(event `self.ReceiveActorEndOverlap`
  (params (OtherActor :type "Actor Object Reference"))
  ;[1 1 1] Comment
  (`KismetSystemLibrary.PrintString` (`KismetSystemLibrary.GetDisplayName` OtherActor)))

(fn `Explode`
  (`KismetSystemLibrary.PrintString` (`KismetStringLibrary.Conv_IntToString` (`KismetArrayLibrary.Array_Length` (`self.GetOverlappingComponents`)))))

(fn `UserConstructionScript`)