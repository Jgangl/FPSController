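; TestBomb is a projectile bomb actor, tagged BombTag at construction, that stops moving when it hits something.
; Calling Shot hides its cube, caches the overlapping components and sets Exploding.
; While Exploding, Tick drops the cube from that list and applies a constant-falloff radial impulse to the rest every frame until a short delay destroys the actor.
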(event `self.ReceiveActorBeginOverlap`
  (params (OtherActor :type "Actor Object Reference")))

(event `self.ReceiveTick`
  (params (DeltaSeconds :type "Float (single-precision)"))
  (bind _objectsinrange (`self.ObjectsInRange`))
  (if (`self.Exploding`)
    (`KismetArrayLibrary.Array_RemoveItem` _objectsinrange (`self.Cube`))
    (`PrimitiveComponent.AddRadialImpulse` _objectsinrange (`self.K2_GetActorLocation`) 200.0 20000.0 "RIF_Constant" false)
    (`KismetSystemLibrary.Delay` 0.2)
    (`self.K2_DestroyActor`)))

(event `self.ReceiveHit`
  (params (MyComp :type "PrimitiveComponent Object Reference") (Other :type "Actor Object Reference") (OtherComp :type "PrimitiveComponent Object Reference") (bSelfMoved :type Boolean) (HitLocation :type "Vector Structure") (HitNormal :type "Vector Structure") (NormalImpulse :type "Vector Structure") (Hit :type "HitResult Structure (by ref)"))
  (`MovementComponent.StopMovementImmediately` (`self.ProjectileMovement`)))

(fn `Shot`
  (`SceneComponent.SetVisibility` (`self.Cube`) false false)
  (set `self.ObjectsInRange` (`self.GetOverlappingComponents`))
  (set `self.Exploding` true))

(fn `UserConstructionScript`
  (set `self.Tags` (`|MakeArray` (`self.bombTag`))))