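; Arrow projectile actor for a bow, which flies with a ProjectileMovement component and stops where it hits.
; Each Tick sets its pitch from the velocity direction, keeping roll and yaw, so the arrow tilts along its flight path.
; On Hit it halts movement, moves to the hit location and prints debug text.
; Disconnected nodes that would spawn a point light, attach it to the hit actor and destroy the arrow never run.
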(event `self.ReceiveTick`
  (params (DeltaSeconds :type "Float (single-precision)"))
  (`self.K2_SetActorRotation` (`KismetMathLibrary.MakeRotator` (.roll (`self.K2_GetActorRotation`)) (.pitch (`KismetMathLibrary.MakeRotFromX` (`self.GetVelocity`))) (.yaw (`self.K2_GetActorRotation`)))))

(event `self.ReceiveHit`
  (params (MyComp :type "PrimitiveComponent Object Reference") (Other :type "Actor Object Reference") (OtherComp :type "PrimitiveComponent Object Reference") (bSelfMoved :type Boolean) (HitLocation :type "Vector Structure") (HitNormal :type "Vector Structure") (NormalImpulse :type "Vector Structure") (Hit :type "HitResult Structure (by ref)"))
  (`KismetSystemLibrary.PrintString` "Hit")
  (`MovementComponent.StopMovementImmediately` (`self.ProjectileMovement`))
  (`KismetSystemLibrary.PrintString` (`KismetStringLibrary.Conv_VectorToString` HitLocation))
  (`self.K2_SetActorLocation` HitLocation))

(fn `UserConstructionScript`)